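; Spawner actor that scatters a list of objects, including counted RealPackages, and can spawn an ExtractionZone on demand.
; Shortly after BeginPlay, if no current object exists, it spawns each listed class at random navigable XY points within a radius taken from the smaller spawn-range axis.
; Objects start at a fixed high Z, ignoring the computed random Z.
; SpawnExtraction uses the same XY sampling with a low, conditionally set height.
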(event `self.ReceiveBeginPlay`
  (bind _x (.x (`self.Randow_Spawn_Range`)))
  (bind _y (.y (`self.Randow_Spawn_Range`)))
  (`|ExecutionSequence`
    (:`then_0`
      (if (> _x _y)
        (set `self.radius` _y)
        (else
          (set `self.radius` _x))))
    (:`then_1`
      (`KismetSystemLibrary.Delay` 0.5)
      (`self.AttemptToSpawn`))))

(event `SpawnExtraction`
  (bind _randomlocation (`NavigationSystemV1.K2_GetRandomLocationInNavigableRadius` (`self.K2_GetActorLocation`) (`self.radius`) null null))
  (`|ExecutionSequence`
    (:`then_1`
      (if (> (`self.z_val_random`) 180.0)
        (bind _output_get (set `self.z_val_random` 0.0))
        (else
          (set `self.z_val_random` 180.0))))
    (:`then_2`
      (`|SpawnActorFromClass` "/Game/Blueprints/ExtractionZone.ExtractionZone_C" (`KismetMathLibrary.MakeTransform` (`KismetMathLibrary.MakeVector` (.x _randomlocation) (.y _randomlocation) _output_get) (`self.K2_GetActorRotation`)) "AdjustIfPossibleButAlwaysSpawn" "OverrideRootScale" self null))))

(fn `AttemptToSpawn`
  (`/Engine/EditorBlueprintResources/StandardMacros.IsValid` (`self.currentObject`)
    (:`Is Not Valid`
      (`self.Spawn`))))

(fn `Spawn`
  (bind (_returnvalue_x _returnvalue_y _returnvalue_z) (`KismetMathLibrary.BreakVector` (`KismetMathLibrary.RandomPointInBoundingBox` (`self.K2_GetActorLocation`) (`self.Randow_Spawn_Range`))))
  (bind _randomlocation (`NavigationSystemV1.K2_GetRandomLocationInNavigableRadius` (`self.K2_GetActorLocation`) (`self.radius`) null null))
  (for _array_element (`self.objectsToSpawn`)
    (`|ExecutionSequence`
      (:`then_0`
        (if (> (`self.z_val_random`) 180.0)
          (set `self.z_val_random` _returnvalue_z)
          (else
            (set `self.z_val_random` 180.0))))
      (:`then_1`
        (bind _returnvalue (`|SpawnActorFromClass` _array_element (`KismetMathLibrary.MakeTransform` (`KismetMathLibrary.MakeVector` (.x _randomlocation) (.y _randomlocation) 2000.0) (`self.K2_GetActorRotation`)) "AdjustIfPossibleButAlwaysSpawn" "OverrideRootScale" self null))
        (if (== (`GameplayStatics.GetObjectClass` _returnvalue) "/Game/Blueprints/Interactibles/RealPackage.RealPackage_C")
          (set `self.realPackageCount` (+ (`self.realPackageCount`) 1)))
        (set `self.currentObject` _returnvalue)))))

(fn `UserConstructionScript`)