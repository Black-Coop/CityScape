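; RealPackage is an interactible pickup that counts toward unlocking extraction.
; On Interaction, it increments the Player_Character's Package count and casts its owner to Spawner.
; When the count reaches the Spawner's RealPackageCount, it calls SpawnExtraction on that Spawner.
; The package then destroys itself, although a failed owner cast stops this after the count has already risen.
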(event `/Game/Blueprints/Interfaces/InteractionInterface.Interaction`
  (params (player :type "Pawn Object Reference"))
  (bind _asplayer_character (cast `/Game/Blueprints/Player_Character` player))
  (bind _output_get (set `/Game/Blueprints/Player_Character.package` (+ (`/Game/Blueprints/Player_Character.package` _asplayer_character) 1) _asplayer_character))
  (bind _asspawner (cast `/Game/Blueprints/ObjectSpawner/Spawner` (`self.GetOwner`)))
  (if (>= _output_get (`/Game/Blueprints/ObjectSpawner/Spawner.realPackageCount` _asspawner))
    (`/Game/Blueprints/ObjectSpawner/Spawner.Spawn Extraction` _asspawner))
  (`self.K2_DestroyActor`))

(fn `UserConstructionScript`
  (`parent.UserConstructionScript`))