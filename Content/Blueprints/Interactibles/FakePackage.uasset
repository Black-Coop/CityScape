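; FakePackage is a booby-trapped interactible package that explodes after a player interacts with it.
; Interaction spawns smoke, waits briefly, then spawns fire, explosion and dust effects before destroying the actor.
; Two sphere traces using DamageRadius send a lighter, then a heavier attack message to the interacting player if hit.
; The first trace and explosion emitter have no location set, unlike the final trace at the package.
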(event `/Game/Blueprints/Interfaces/InteractionInterface.Interaction`
  (params (player :type "Pawn Object Reference"))
  (bind _returnvalue (`self.K2_GetActorRotation`))
  (bind _returnvalue_2 (`self.K2_GetActorLocation`))
  (`GameplayStatics.SpawnEmitterAtLocation` "/Game/Particles/P_Smoke.P_Smoke" _returnvalue_2 _returnvalue (0.6 0.6 0.6) true "AutoRelease")
  (`KismetSystemLibrary.Delay` 2.0)
  (`GameplayStatics.SpawnEmitterAtLocation` "/Game/Particles/P_Fire.P_Fire" _returnvalue_2 _returnvalue (0.5 0.5 0.5))
  (bind _outhit (`KismetSystemLibrary.SphereTraceSingle` (0.0 0.0 0.0) (0.0 0.0 0.0) (`self.damageRadius`) "TraceTypeQuery2" false (`|MakeArray` null :!type "Actor Object Reference") "Persistent"))
  (if (== player (`.HitActor` (`GameplayStatics.BreakHitResult` _outhit)))
    (message `/Game/Blueprints/Interfaces/ArmedPawnInterface.RecieveAttack` player 25.0))
  (`GameplayStatics.SpawnEmitterAtLocation` "/Game/Particles/P_Explosion.P_Explosion" (0.0 0.0 0.0) _returnvalue (1.0 1.0 1.0) true "AutoRelease")
  (`GameplayStatics.SpawnEmitterAtLocation` "/Game/Particles/P_Ambient_Dust.P_Ambient_Dust" _returnvalue_2 _returnvalue (0.5 0.5 0.5) true "AutoRelease")
  ;[1 1 1] Explosion
  (bind _outhit_2 (`KismetSystemLibrary.SphereTraceSingle` _returnvalue_2 _returnvalue_2 (`self.damageRadius`) "TraceTypeQuery2" false (`|MakeArray` null :!type "Actor Object Reference")))
  (if (== player (`.HitActor` (`GameplayStatics.BreakHitResult` _outhit_2)))
    (message `/Game/Blueprints/Interfaces/ArmedPawnInterface.RecieveAttack` player 100.0))
  (`self.K2_DestroyActor`))

(fn `UserConstructionScript`
  (`parent.UserConstructionScript`))