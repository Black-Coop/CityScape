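; ActionHUD is the in-game HUD that creates the action-time widgets and a pause menu and switches between them.
; On BeginPlay it adds crosshair, timer, package counter, ammo and grapple telemetry widgets to the viewport, storing them in an array, plus a hidden pause menu.
; ActivateResumeMenu calls ShowActionTimeHUDElements, which swaps visibility between that array and the pause menu and toggles game-only or UI-only input.
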(event `self.ReceiveBeginPlay`
  (bind _returnvalue (`|CreateWidget` "/Game/Blueprints/HUD_and_Widgets/CrossHair.CrossHair_C"))
  (`UserWidget.AddToViewport` _returnvalue 0)
  (bind _returnvalue_2 (`|CreateWidget` "/Game/Blueprints/HUD_and_Widgets/TimerWidget.TimerWidget_C"))
  (`UserWidget.AddToViewport` _returnvalue_2 0)
  (bind _returnvalue_3 (`|CreateWidget` "/Game/Blueprints/HUD_and_Widgets/PackageCounterWidget.PackageCounterWidget_C"))
  (`UserWidget.AddToViewport` _returnvalue_3 0)
  (bind _returnvalue_4 (`|CreateWidget` "/Game/Blueprints/HUD_and_Widgets/AmmoCount.AmmoCount_C"))
  (`UserWidget.AddToViewport` _returnvalue_4 0)
  (bind _returnvalue_5 (`|CreateWidget` "/Game/Blueprints/HUD_and_Widgets/Grapple_Telemetry_Widget.Grapple_Telemetry_Widget_C"))
  (`UserWidget.AddToViewport` _returnvalue_5 0)
  (set `self.ActionTimeHUDElements` (`|MakeArray` _returnvalue _returnvalue_2 _returnvalue_3 _returnvalue_4 _returnvalue_5 :!type "UserWidget Object Reference"))
  (bind _returnvalue_6 (`|CreateWidget` "/Game/Blueprints/HUD_and_Widgets/PauseMenu.PauseMenu_C"))
  (bind _output_get (set `self.PauseWidget` _returnvalue_6))
  (`Widget.SetVisibility` _output_get "Hidden")
  (`UserWidget.AddToViewport` _output_get 0))

(event `ActivateResumeMenu`
  (params (show :type Boolean))
  (`self.ShowActionTimeHUDElements` show))

(fn `ShowActionTimeHUDElements`
  (params (shouldShow :type Boolean))
  (if shouldShow
    (for _array_element (`self.ActionTimeHUDElements`)
      (`Widget.SetVisibility` _array_element "Visible"))
    (`Widget.SetVisibility` (`self.PauseWidget`) "Hidden")
    (`WidgetBlueprintLibrary.SetInputMode_GameOnly` (`GameplayStatics.GetPlayerController` 0))
    (else
      (for _array_element_2 (`self.ActionTimeHUDElements`)
        (`Widget.SetVisibility` _array_element_2 "Hidden"))
      (`Widget.SetVisibility` (`self.PauseWidget`) "Visible")
      (`WidgetBlueprintLibrary.SetInputMode_UIOnlyEx` (`GameplayStatics.GetPlayerController` 0) null))))

(fn `UserConstructionScript`)