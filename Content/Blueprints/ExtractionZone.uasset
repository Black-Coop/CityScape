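; Extraction zone actor that ends the mission successfully when the player character enters it.
; On overlap with a Player_Character it waits two seconds, pauses the game, and shows the ActionHUD game over menu flagged as mission success.
; An invalid player controller only prints a debug message.
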(event `self.ReceiveBeginPlay`)

(event `self.ReceiveActorBeginOverlap`
  (params (OtherActor :type "Actor Object Reference"))
  (bind _asplayer_character (cast `/Game/Blueprints/Character/Player_Character` OtherActor))
  (`self.PlayerEnteredEZ` _asplayer_character))

(event `self.ReceiveActorEndOverlap`
  (params (OtherActor :type "Actor Object Reference")))

(event `PlayerEnteredEZ`
  (params (player :type "Character Object Reference"))
  (bind _returnvalue (`Pawn.GetController` player))
  (`KismetSystemLibrary.Delay` 2.0)
  (`GameplayStatics.SetGamePaused` true)
  (`/Engine/EditorBlueprintResources/StandardMacros.IsValid` _returnvalue
    (:`Is Valid`
      (bind _asplayer_controller (cast `PlayerController` _returnvalue))
      (bind _asaction_hud (cast `/Game/HUD_and_Widgets/ActionHUD` (`PlayerController.GetHUD` _asplayer_controller)))
      (`/Game/HUD_and_Widgets/ActionHUD.ActivateGameOverMenu` _asaction_hud true true))
    (:`Is Not Valid`
      (`KismetSystemLibrary.PrintString` "Somehow It is not valid" true true (struct :`R` 1.0 :`G` 0.328145 :`B` 0.661216 :`A` 1.0)))))

(fn `UserConstructionScript`)