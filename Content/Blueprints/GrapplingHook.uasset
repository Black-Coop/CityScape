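; Player-held gun actor that combines a swinging grappling hook with hitscan shooting and magazine reloading.
; A trace from the gun socket sets the hook point and rope length.
; While hooked, Tick aims gun and cable at it, pulling the parent back within range and adding a velocity-dot-product force for swinging.
; Releasing pushes the character forward, Launch flings it toward the hook on a timeline cooldown, and camera traces damage enemies.
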(event `Event ShootCable`
  ;[1 1 1] Shoot and Retract Cable
  (`self.ShootCableRaycast`))

(event `self.ReceiveBeginPlay`
  ;[1 1 1] Begin Play
  (set `self.HookRange` 10000.0)
  (set `self.hookActive` false)
  (set `self.hookLocation` (`SceneComponent.K2_GetComponentLocation` (`self.GunMesh`)))
  (bind _output_get (set `self.magazineAmmo` 20))
  (`TextRenderComponent.K2_SetText` (`self.ClipCountText`) (`KismetTextLibrary.Conv_IntToText` _output_get)))

(event `Event ResetCable`
  ;[1 1 1] Shoot and Retract Cable
  (if (`self.hookActive`)
    (`self.ResetCableToUnhooked`)
    (`self.addForwardPush`)))

(event `self.ReceiveTick`
  (params (DeltaSeconds :type "Float (single-precision)"))
  (bind (_parentisplayer _parentactorobject) (`self.GetParentActorAndAssert`))
  ;[1 1 1] Event Tick
  (if _parentisplayer
    (if (`self.hookActive`)
      (`self.Event LocationAdjust`)
      (set `self.previousFramePosition` (`self.K2_GetActorLocation` _parentactorobject))
      (else
        (`self.FixRotation`)))))

(event `Event LocationAdjust`
  ;[1 1 1] AdjustPositioning
  (`self.adjustCable`)
  (`self.turnGunToGrappleRotation`)
  (if (not (`.isInsideRange` (`self.distanceBetweenCharacterAndHookPosition`)))
    (`self.Apply Thether` (`.ParentActorObject` (`self.GetParentActorAndAssert`)))
    (`self.DotProductOfVelocity`)))

(event `Event Launch`
  (bind (_parentisplayer _parentactorobject) (`self.GetParentActorAndAssert`))
  ;[1 1 1] Launch character
  (if (and (`self.hookActive`) (`self.isLaunchAvailable`))
    (bind _ascharacter (cast `Character` _parentactorobject))
    (`Character.LaunchCharacter` _ascharacter (+ (* (* (`KismetMathLibrary.Normal` (- (`self.hookLocation`) (`self.K2_GetActorLocation` _parentactorobject))) 3.0) 1000.0) (0.0 0.0 600.0)) false false)
    (set `self.isLaunchAvailable` false)
    (`self.ResetCableToUnhooked`)
    (`Timeline|Timeline_0` :!via `PlayFromStart`
      (:`Finished`
        (set `self.isLaunchAvailable` true)))))

(event `Event FireBullet`
  (if (!= (`self.magazineAmmo`) 0)
    (`|ExecutionSequence`
      (:`then_0`
        (`self.FireWeapon`)))
    (else
      (`self.reloadAmmo` :!label _label))))

(event `Event ReloadGun`
  (goto _label))

(fn `addForwardPush`
  (bind _ascharacter (cast `Character` (`.ParentActorObject` (`self.GetParentActorAndAssert`))))
  (`Character.LaunchCharacter` _ascharacter (* (`KismetMathLibrary.GetForwardVector` (`self.K2_GetActorRotation` _ascharacter)) 1500.0) false false))

(fn `adjustCable`
  (bind _hooklocation (`self.hookLocation`))
  (bind _returnvalue (`SceneComponent.GetSocketLocation` (`self.GunMesh`) "GrappleSocket"))
  (`SceneComponent.K2_SetWorldLocationAndRotation` (`self.Cable`) (`KismetMathLibrary.VInterpTo` _returnvalue _hooklocation (`GameplayStatics.GetWorldDeltaSeconds`) (`self.interpolationSpeed`)) (`KismetMathLibrary.FindLookAtRotation` _returnvalue _hooklocation) true false)
  (return))

(fn `Apply Thether`
  (params (AttachedActor :type "Actor Object Reference"))
  (bind _returnvalue (`self.K2_GetActorLocation` AttachedActor))
  (bind _ropelength (`self.ropeLength`))
  (bind _returnvalue_2 (`KismetMathLibrary.VSize` (`self.GrappleSocketToHookLocationVector`)))
  (if (>= _returnvalue_2 _ropelength)
    (`self.K2_SetActorLocation` AttachedActor (`KismetMathLibrary.VInterpTo` _returnvalue (+ (* (* (`KismetMathLibrary.Normal` (- (`self.hookLocation`) _returnvalue)) 1.0) (- _returnvalue_2 _ropelength)) _returnvalue) (`GameplayStatics.GetWorldDeltaSeconds`) (`self.interpolationSpeed`)) false false)
    (return)))

(fn `AttachToActor`
  (params (SocketName :type Name) (ParentActor :type "Actor Object Reference"))
  (`self.K2_AttachToActor` ParentActor SocketName "KeepWorld" "KeepWorld" "KeepWorld" false)
  (return))

(fn `DotProductOfVelocity`
  (bind (_parentisplayer _parentactorobject) (`self.GetParentActorAndAssert`))
  (bind _returnvalue (- (`self.hookLocation`) (`SceneComponent.GetSocketLocation` (`self.GunMesh`) "GrappleSocket")))
  (if _parentisplayer
    (`CharacterMovementComponent.AddForce` (`self.GetComponentByClass` _parentactorobject "/Script/Engine.CharacterMovementComponent") (* (* (`KismetMathLibrary.Normal` _returnvalue) (`KismetMathLibrary.Dot_VectorVector` (`self.GetVelocity` _parentactorobject) _returnvalue)) -1.0))
    (return)))

(fn `FireWeapon`
  (bind _returnvalue (`GameplayStatics.GetPlayerCameraManager` 0))
  (bind _returnvalue_2 (`PlayerCameraManager.GetCameraLocation` _returnvalue))
  ;[1 1 1] Fire Bullet and Reload
  (bind _outhit (`KismetSystemLibrary.LineTraceSingle` :`Start` _returnvalue_2 :`End` (+ _returnvalue_2 (* (`KismetMathLibrary.Conv_RotatorToVector` (`PlayerCameraManager.GetCameraRotation` _returnvalue)) (`self.WeaponRange`))) :`TraceChannel` "TraceTypeQuery2" :`DrawDebugType` "ForOneFrame"))
  (`|ExecutionSequence`
    (:`then_0`
      (bind _asenemy_base_character (cast `/Game/Blueprints/AI/Blueprint/EnemyBaseCharacter` (`.HitActor` (`GameplayStatics.BreakHitResult` _outhit))))
      (message `/Game/Blueprints/Interfaces/ArmedPawnInterface.RecieveAttack` _asenemy_base_character 100.0))
    (:`then_1`
      (bind _result (`/Engine/EditorBlueprintResources/StandardMacros.DecrementInt` (`self.magazineAmmo`))
        (:`  `
          (`self.SetAmmoText` _result)
          (if (== _result 0)
            (`self.reloadAmmo`)))))))

(fn `FixRotation`
  (`self.K2_SetActorRotation` (`PlayerCameraManager.GetCameraRotation` (`GameplayStatics.GetPlayerCameraManager` 0))))

(fn `reloadAmmo`
  (bind _totalammo (`self.totalAmmo`))
  (bind _magazineammo (`self.magazineAmmo`))
  (bind _magazinesize (`self.magazineSize`))
  (bind _returnvalue (- _magazinesize _magazineammo))
  (if (>= _totalammo _returnvalue)
    (set `self.totalAmmo` (- _totalammo _returnvalue))
    (set `self.magazineAmmo` _magazinesize)
    (`self.SetAmmoText` _magazineammo)
    (else
      (set `self.magazineAmmo` (+ _totalammo _magazineammo))
      (set `self.totalAmmo` 0)
      (`self.SetAmmoText` _magazineammo))))

(fn `ResetCableToUnhooked`
  (bind _cable (`self.Cable`))
  (set `CableComponent.CableLength` 0.0 _cable)
  (`SceneComponent.SetVisibility` _cable false true)
  (set `self.hookActive` false)
  (set `self.ropeLength` 0.0)
  (set `self.hookLocation` (`self.K2_GetActorLocation`))
  (return))

(fn `ShootCableRaycast`
  (bind (_parentisplayer _parentactorobject) (`self.GetParentActorAndAssert`))
  (bind _gunmesh (`self.GunMesh`))
  (bind _cable (`self.Cable`))
  (bind _returnvalue (`SceneComponent.GetSocketLocation` _gunmesh "GrappleSocket"))
  (bind _returnvalue_2 (`SceneComponent.GetSocketLocation` (`self.GunMesh`) "GrappleSocket"))
  (if _parentisplayer
    (bind (_outhit _returnvalue_3) (`KismetSystemLibrary.LineTraceSingle` _returnvalue (+ _returnvalue (* (`KismetMathLibrary.GetForwardVector` (`SceneComponent.GetSocketRotation` _gunmesh "GrappleSocket")) (`self.HookRange`))) "TraceTypeQuery1" false (`|MakeArray` _parentactorobject) "ForOneFrame"))
    (if _returnvalue_3
      (bind _output_get (set `self.hookLocation` (`.Location` (`GameplayStatics.BreakHitResult` _outhit))))
      (bind _output_get_2 (set `CableComponent.CableLength` (+ (`KismetMathLibrary.VSize` (- _output_get _returnvalue_2)) (`KismetMathLibrary.VSize` (- _returnvalue_2 (`self.K2_GetActorLocation` _parentactorobject))) 5.0) _cable))
      (`SceneComponent.K2_SetWorldLocationAndRotation` _cable (`KismetMathLibrary.VInterpTo` _returnvalue_2 _output_get (`GameplayStatics.GetWorldDeltaSeconds`) (`self.interpolationSpeed`)) (`KismetMathLibrary.FindLookAtRotation` _returnvalue_2 _output_get) true false)
      (`SceneComponent.SetVisibility` _cable true false)
      (set `self.hookActive` true)
      (set `self.ropeLength` _output_get_2)
      (return)
      (else
        (set `self.hookLocation` (`self.K2_GetActorLocation`))))))

(fn `turnGunToGrappleRotation`
  (`self.K2_SetActorRotation` (`SceneComponent.K2_GetComponentRotation` (`self.Cable`))))

(fn `UserConstructionScript`)