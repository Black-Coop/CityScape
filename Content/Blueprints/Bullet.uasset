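; Bullet projectile actor that damages the pawns it hits.
; On overlap it ignores actors of the shooter's exact class, destroys itself on static mesh actors, and sends pawns an attack message with its damage and instigator before destroying itself.
; Other overlapped actors are passed through.
; Tick accumulates travelled distance from the projectile movement velocity and destroys the bullet at a fixed maximum range.
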(event `self.ReceiveActorBeginOverlap`
  (params (OtherActor :type "Actor Object Reference"))
  (if (not (== (`GameplayStatics.GetObjectClass` OtherActor) (`self.ShooterClassType`)))
    (cast `StaticMeshActor` OtherActor
      (:`then`
        _)
      (:`CastFailed`
        (bind _aspawn (cast `Pawn` OtherActor))
        (message `/Game/Blueprints/Interfaces/ArmedPawnInterface.RecieveAttack` _aspawn (`self.bulletDamage`) (`self.GetInstigator`))))
    (`self.K2_DestroyActor`)))

(event `self.ReceiveTick`
  (params (DeltaSeconds :type "Float (single-precision)"))
  (bind _output_get (set `self.distanceCovered` (+ (`self.distanceCovered`) (`KismetMathLibrary.VSize` (* (`MovementComponent.Velocity` (`self.ProjectileMovement`)) DeltaSeconds)))))
  (if (>= _output_get 20000.0)
    (`self.K2_DestroyActor`)))

(fn `UserConstructionScript`)