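; Patrol checkpoint actor that spawns enemy pawns and tracks how many are registered to it against a patrol limit.
; On BeginPlay it spawns one pawn per limit slot at random navigable nearby X/Y points and a fixed height, each with a default controller.
; Register, deregister and limit-check functions maintain the pawn list and count.
; Tick writes the count and limit to a text display.
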(event `self.ReceiveBeginPlay`
  (bind _randomlocation (`NavigationSystemV1.K2_GetRandomLocationInNavigableRadius` (`self.K2_GetActorLocation`) 500.0 null null))
  (for _ (range (`self.patrolLimit`))
    (bind _returnvalue (`|SpawnActorFromClass` (`self.EnemyPawn_Class_Reference`) (`KismetMathLibrary.MakeTransform` (`KismetMathLibrary.MakeVector` (.x _randomlocation) (.y _randomlocation) 500.0)) "AdjustIfPossibleButDontSpawnIfColliding" "OverrideRootScale" null null))
    (`Pawn.SpawnDefaultController` _returnvalue)
    (`KismetSystemLibrary.PrintString` (`KismetSystemLibrary.GetDisplayName` _returnvalue))))

(event `self.ReceiveTick`
  (params (DeltaSeconds :type "Float (single-precision)"))
  (`TextRenderComponent.K2_SetText` (`self.PatrolCountText`) (`KismetTextLibrary.Conv_StringToText` (`KismetStringLibrary.Concat_StrStr` (`KismetStringLibrary.Conv_IntToString` (`self.patrolCount`)) "/" (`KismetStringLibrary.Conv_IntToString` (`self.patrolLimit`))))))

(fn `Check Limit`
  (returns (isAvailable :type Boolean))
  (if (> (`self.patrolLimit`) (`self.patrolCount`))
    (return true)
    (else
      (return false))))

(fn `Patrol Deregister Target`
  (params (pawnToDeregister :type "Pawn Object Reference"))
  (bind _returnvalue (`KismetArrayLibrary.Array_RemoveItem` (`self.PatrolsRegistered`) pawnToDeregister))
  (if _returnvalue
    (`/Engine/EditorBlueprintResources/StandardMacros.DecrementInt` (`self.patrolCount`)
      (:`  `
        (return)))))

(fn `Patrol Register Target`
  (params (pawnToRegister :type "Pawn Object Reference"))
  (returns (isRegistered :type Boolean))
  (if (> (`self.patrolLimit`) (`self.patrolCount`))
    (`/Engine/EditorBlueprintResources/StandardMacros.IncrementInt` (`self.patrolCount`)
      (:`  `
        (`KismetArrayLibrary.Array_Add` (`self.PatrolsRegistered`) pawnToRegister)
        (return true)))
    (else
      (return false))))

(fn `UserConstructionScript`)