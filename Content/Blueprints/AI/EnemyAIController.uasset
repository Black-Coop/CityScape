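; AI controller that sends an enemy patrolling between PatrolCheckpoint actors, driven by a behavior tree.
; On BeginPlay it gathers all checkpoints, seeds the blackboard, picks a first target and runs the tree.
; Target selection seeks the nearest checkpoint within range that passes its limit check and differs from the starting one, then registers the pawn there.
; Recalculation deregisters the pawn from its current target, stores it as the start and searches again.
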(event `self.ReceiveBeginPlay`
  (bind _outactors (`GameplayStatics.GetAllActorsOfClass` "/Game/Blueprints/AI/PatrolCheckpoint.PatrolCheckpoint_C"))
  (set `self.patrolCheckpoints` _outactors)
  (bind _blackboardcomponent (`self.UseBlackboard` "/Game/Blueprints/AI/Blackboard.Blackboard"))
  (bind _output_get (set `self.BlackboardComponent` _blackboardcomponent))
  (`BlackboardComponent.SetValueAsFloat` _output_get "patrolLength" 10000.0)
  (`BlackboardComponent.SetValueAsVector` _output_get "patrolBeginPosition" (`self.K2_GetActorLocation` (`self.K2_GetPawn`)))
  (`self.findClosestCheckpoint`)
  (`self.RunBehaviorTree` "/Game/Blueprints/AI/BehaviourTree.BehaviourTree"))

(event `RecalculateCheckpointTarget`
  (bind _returnvalue (`self.K2_GetPawn`))
  (bind _aspatrol_checkpoint (cast `/Game/Blueprints/AI/PatrolCheckpoint` (`BlackboardComponent.GetValueAsObject` (`AIBlueprintHelperLibrary.GetBlackboard` _returnvalue) "patrolTargetCheckpoint")))
  (`self.setBeginCheckpoint` _returnvalue _aspatrol_checkpoint)
  (`self.findClosestCheckpoint`))

(fn `findClosestCheckpoint`
  (locals (minLength :type "Float (double-precision)" :default -10.0) (index :type Integer))
  (bind _returnvalue (`self.K2_GetPawn`))
  (bind _minlength (`local.minLength`))
  (bind _output (`|GetArrayItem` (`self.patrolCheckpoints`) (`local.index`)))
  (for (_array_element _array_index) (`self.patrolCheckpoints`)
    (if (> (`self.targetCheckpointDistanceLimit`) (`KismetMathLibrary.VSize` (- (`self.K2_GetActorLocation` (`self.K2_GetPawn`)) (`self.K2_GetActorLocation` _array_element))))
      (bind _isavailable (`/Game/Blueprints/AI/PatrolCheckpoint.Check Limit` _array_element))
      (bind _returnvalue_2 (`self.Not Equal` _array_element (`self.getBeginningCheckpoint`)))
      (bind _returnvalue_3 (`KismetMathLibrary.VSize` (- (`self.K2_GetActorLocation` _array_element) (`self.K2_GetActorLocation` _returnvalue))))
      (if (and _isavailable _returnvalue_2 (or (>= _minlength _returnvalue_3) (<= _minlength -1.0)))
        (set `local.minLength` _returnvalue_3)
        (set `local.index` _array_index))))
  (bind _isregistered (`/Game/Blueprints/AI/PatrolCheckpoint.Patrol Register Target` _output _returnvalue))
  (if _isregistered
    (`BlackboardComponent.SetValueAsObject` (`self.BlackboardComponent`) "patrolTargetCheckpoint" _output)))

(fn `Not Equal`
  (params (A :type "Object Object Reference") (B :type "Object Object Reference"))
  (returns (ReturnValue :type Boolean))
  (return (or (!= A B) (not (`KismetSystemLibrary.IsValid` B)))))

(fn `setBeginCheckpoint`
  (params (pawnToActOn :type "Pawn Object Reference") (beginCheckpointToSet :type "/Game/Blueprints/AI/PatrolCheckpoint Object Reference"))
  (`/Game/Blueprints/AI/PatrolCheckpoint.Patrol Deregister Target` beginCheckpointToSet pawnToActOn)
  (`BlackboardComponent.SetValueAsObject` (`AIBlueprintHelperLibrary.GetBlackboard` pawnToActOn) "patrolBeginCheckpoint" beginCheckpointToSet)
  (return))

(fn `UserConstructionScript`)