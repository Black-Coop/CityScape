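; Base enemy AI character that senses targets, fires bullets and is destroyed when damage exceeds its health.
; AI perception updates feed blackboard keys for target, visibility and last known position, while toggling an alert cube and movement speed.
; On sight loss, a timeline acts as a grace period before clearing the target and slowing down.
; Shoot spawns a bullet at a socket with random angular spread, ignoring its Difficulty input.
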(event `self.ReceiveBeginPlay`
  (bind _output_get (set `self.blackBoard` (`AIBlueprintHelperLibrary.GetBlackboard` (`AIBlueprintHelperLibrary.GetAIController` self))))
  (set `CharacterMovementComponent.MaxWalkSpeed` 300.0 (`self.CharacterMovement`))
  (`BlackboardComponent.SetValueAsFloat` _output_get "maxShootingDistanceBetweenCharacterAndEnemy" (`self.shootingRange`)))

(event `self.AIPerception.OnTargetPerceptionUpdated`
  (params (Actor :type "Actor Object Reference") (Stimulus :type "AIStimulus Structure"))
  (bind (_age _expirationage _strength _stimuluslocation _receiverlocation _tag _bsuccessfullysensed) (break `AIStimulus` Stimulus))
  (bind _alertedcube (`self.AlertedCube`))
  (bind _blackboard (`self.blackBoard`))
  (bind _blackboard_2 (`self.blackBoard`))
  (if _bsuccessfullysensed
    (`BlackboardComponent.SetValueAsObject` _blackboard "targetActor" Actor)
    (`BlackboardComponent.SetValueAsVector` _blackboard "lastKnownPlayerPosition" _stimuluslocation)
    (`BlackboardComponent.SetValueAsBool` _blackboard "canSeePlayer" true)
    (`SceneComponent.SetVisibility` _alertedcube true false)
    (`BlackboardComponent.SetValueAsBool` (`self.blackBoard`) "isTargetSightActive" true)
    (set `CharacterMovementComponent.MaxWalkSpeed` 600.0 (`self.CharacterMovement`))
    (else
      (`BlackboardComponent.SetValueAsVector` _blackboard "lastKnownPlayerPosition" _stimuluslocation)
      (`BlackboardComponent.SetValueAsBool` _blackboard "canSeePlayer" false)
      (`SceneComponent.SetVisibility` _alertedcube false false)
      (`Timeline|Timeline_0` :!via `PlayFromStart`
        (:`Finished`
          (`BlackboardComponent.SetValueAsBool` _blackboard_2 "isTargetSightActive" false)
          (`BlackboardComponent.SetValueAsObject` _blackboard_2 "targetActor" null)
          (set `CharacterMovementComponent.MaxWalkSpeed` 300.0 (`self.CharacterMovement`)))))))

(event `/Game/Blueprints/Interfaces/DamagableInterface.ReduceHealth`
  (params (DamageAmount :type "Float (single-precision)"))
  (bind _health (`self.health`))
  (if (< _health DamageAmount)
    (`/Game/Blueprints/Interfaces/DamagableInterface.Die`)
    (else
      (set `self.health` (- _health DamageAmount)))))

(event `/Game/Blueprints/Interfaces/DamagableInterface.Die`
  (`self.K2_DestroyActor`))

(event `/Game/Blueprints/Interfaces/ArmedPawnInterface.RecieveAttack`
  (params (DamageAmount :type "Float (single-precision)"))
  (`/Game/Blueprints/Interfaces/DamagableInterface.ReduceHealth` DamageAmount)
  (`KismetSystemLibrary.PrintText` "RecievedAttack"))

(fn `Shoot`
  (params (difficulty :type Byte))
  (returns (success :type Boolean))
  (bind _returnvalue (`SceneComponent.GetSocketTransform` (`self.BulletShootPoint`) "BulletSocket" "RTS_World"))
  (bind _returnvalue_2 (`|SpawnActorFromClass` "/Game/Blueprints/Bullet.Bullet_C" (`KismetMathLibrary.MakeTransform` (.location _returnvalue) (`KismetMathLibrary.MakeRotator` (`KismetMathLibrary.RandomFloatInRange` (- (.roll (.rotation _returnvalue)) 5.0) (+ (.roll (.rotation _returnvalue)) 5.0)) (`KismetMathLibrary.RandomFloatInRange` (- (.pitch (.rotation _returnvalue)) 5.0) (+ (.pitch (.rotation _returnvalue)) 5.0)) (`KismetMathLibrary.RandomFloatInRange` (- (.yaw (.rotation _returnvalue)) 5.0) (+ 0.0 (.yaw (.rotation _returnvalue))))) (.scale _returnvalue)) "AdjustIfPossibleButDontSpawnIfColliding" "OverrideRootScale" null null))
  (return (`KismetSystemLibrary.IsValid` _returnvalue_2)))

(fn `UserConstructionScript`)